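; BP_LevelPath is a spline path actor that moves a given character along its points one segment at a time.
; MoveCharacterAlongSpline plays a timeline whose alpha lerps between the spline distances of the current and next point, setting the character's location with sweep.
; When each segment finishes, it increments the point index, waits briefly, then calls itself again until the last point is reached.
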(event `MoveCharacterAlongSpline`
  (params (Character :type "/Game/FirstPersonBP/BP_VRPawn Object Reference"))
  (if (< (`self.CurrentPointIndex`) (- (`SplineComponent.GetNumberOfSplinePoints` (`self.Spline`)) 1))
    (bind (_direction _alpha) (`Timeline|CharacterMovementTimeline` :!via `PlayFromStart`)
      (:`Update`
        (`self.K2_SetActorLocation` Character (`SplineComponent.GetLocationAtDistanceAlongSpline` (`self.Spline`) (`KismetMathLibrary.Lerp` (`SplineComponent.GetDistanceAlongSplineAtSplinePoint` (`self.Spline`) (`self.CurrentPointIndex`)) (`SplineComponent.GetDistanceAlongSplineAtSplinePoint` (`self.Spline`) (+ (`self.CurrentPointIndex`) 1)) _alpha) "World") true false))
      (:`Finished`
        (`/Engine/EditorBlueprintResources/StandardMacros.IncrementInt` (`self.CurrentPointIndex`)
          (:`  `
            (`KismetSystemLibrary.Delay` 2.0)
            (`self.MoveCharacterAlongSpline` Character)))))))

(fn `UserConstructionScript`)