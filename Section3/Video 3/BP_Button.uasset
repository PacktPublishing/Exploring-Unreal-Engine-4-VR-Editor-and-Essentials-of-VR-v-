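; BP_Button is an interactable button actor whose cylinder slides when pressed.
; On the first OnInteract event, a DoOnce gate stores the cylinder's world location and computes a target offset by MoveUnits along world X.
; A timeline then lerps the cylinder between the two points.
; The gate is never reset here, so the button works only once.
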(event `/Game/FirstPersonBP/BPI_Interaction.OnInteract`
  (`/Engine/EditorBlueprintResources/StandardMacros.DoOnce` false
    (:`Completed`
      (bind _output_get (set `self.InitialLocation` (`SceneComponent.K2_GetComponentLocation` (`self.Cylinder`))))
      (set `self.TargetLocation` (`KismetMathLibrary.MakeVector` (+ (.x _output_get) (`self.MoveUnits`)) (.y _output_get) (.z _output_get)))
      (bind (_direction _alpha) (`Timeline|PressButtonTimeline` :!via `PlayFromStart`)
        (:`Update`
          (`SceneComponent.K2_SetWorldLocation` (`self.Cylinder`) (`KismetMathLibrary.VLerp` (`self.InitialLocation`) (`self.TargetLocation`) _alpha) false false))))))

(fn `UserConstructionScript`)